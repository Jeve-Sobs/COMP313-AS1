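; Shooter game mode that runs escalating waves of Grux enemies and shows the win UI once the final wave is cleared.
; Each wave's enemy count scales with its number, split between two spawn points by delayed events that re-call themselves.
; Reported kills count down to the next wave, which drops an ammo crate at a random location and shows the wave UI before spawning.
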(event `SetMaxWave`
  (params (WaveMax :type Integer))
  ;[1 1 1] Set Number of Waves
  (set `self.WaveMax` WaveMax))

(event `self.ReceiveBeginPlay`
  ;[1 1 1] Start Game
  (`self.Start Game`))

(event `Start Game`
  ;[1 1 1] Start Game
  (`self.Spawn Wave`))

(event `StartWave`
  ;[1 1 1] Show Wave UI
  (`self.Spawn Ammo`)
  (bind _asbp_first_person_character (cast `/Game/_Main/Blueprints/BP_FirstPersonCharacter` (`GameplayStatics.GetPlayerCharacter` 0)))
  (`/Game/_Main/Blueprints/BP_FirstPersonCharacter.Show Wave UI` _asbp_first_person_character (`self.WaveCur`))
  (`KismetSystemLibrary.Delay` 5.0)
  (`self.Spawn Wave`))

(event `Spawn Wave`
  ;[1 1 1] Spawn Wave
  (bind _output_get (set `self.EnemyNum` (* (`self.WaveCur`) 4)))
  (set `self.EnemyLeft` _output_get)
  (for _index (range (+ _output_get 1))
    (if (> (mod _index 2) 0)
      (`self.Spawn Evemy1`)
      (else
        (`self.Spawn Enemy2`)))))

(event `EnemyKilled`
  ;[1 1 1] Enemy Killed
  (bind _result (`/Engine/EditorBlueprintResources/StandardMacros.DecrementInt` (`self.EnemyLeft`))
    (:`  `
      (if (== _result 0)
        (`self.Increase Wave`)))))

(event `Increase Wave`
  ;[1 1 1] Update Wave
  (set `self.EnemySpawned1` 0)
  (set `self.EnemySpawned2` 0)
  (if (== (`self.WaveMax`) (`self.WaveCur`))
    (`self.Player Wins`)
    (else
      (`/Engine/EditorBlueprintResources/StandardMacros.IncrementInt` (`self.WaveCur`)
        (:`  `
          (`self.StartWave`))))))

(event `Spawn Evemy1`
  ;[1 1 1] Spawns Enemy Logic
  (`KismetSystemLibrary.Delay` 3.0)
  (`/Engine/EditorBlueprintResources/StandardMacros.IncrementInt` (`self.EnemySpawned1`)
    (:`  `
      (`|SpawnActorFromClass` "/Game/_Main/Enemy/BP_Grux.BP_Grux_C" (`self.Spawn Location1`) "Undefined" "OverrideRootScale" null null)
      (if (< (`self.EnemySpawned1`) (/ (`self.EnemyNum`) 2))
        (`self.Spawn Evemy1`)))))

(event `Spawn Enemy2`
  ;[1 1 1] Spawns Enemy Logic
  (`KismetSystemLibrary.Delay` 3.0)
  (`/Engine/EditorBlueprintResources/StandardMacros.IncrementInt` (`self.EnemySpawned2`)
    (:`  `
      (`|SpawnActorFromClass` "/Game/_Main/Enemy/BP_Grux.BP_Grux_C" (`self.SpawnLocation2`) "Undefined" "OverrideRootScale" null null)
      (if (< (`self.EnemySpawned2`) (/ (`self.EnemyNum`) 2))
        (`self.Spawn Enemy2`)))))

(event `Player Wins`
  ;[1 1 1] Win Screen
  (bind _asbp_first_person_character (cast `/Game/_Main/Blueprints/BP_FirstPersonCharacter` (`GameplayStatics.GetPlayerCharacter` 0)))
  (`/Game/_Main/Blueprints/BP_FirstPersonCharacter.ShowWinUI` _asbp_first_person_character))

(event `Spawn Ammo`
  ;[1 1 1] Spawn Ammo crates
  (`|SpawnActorFromClass` "/Game/_Main/Blueprints/BP_Ammo.BP_Ammo_C" (`KismetMathLibrary.MakeTransform` (`|GetArrayItem` (`self.Ammo Crate Location`) (`KismetMathLibrary.RandomInteger` 2))) "Undefined" "OverrideRootScale" null null))

(fn `UserConstructionScript`)