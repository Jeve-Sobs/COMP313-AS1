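; Grux melee enemy for a shooter mode that chases the player and attacks on reach.
; A self-restarting AIMoveTo loop leads into an attack montage whose notify triggers a sphere overlap to damage the player.
; Pawn sensing sets its run speed on sight.
; Point damage plays hit reactions or, at zero health, a random death montage, then loosens collision, reports the kill to GameModeShooter and destroys the actor after a delay.
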(event `self.PawnSensing.OnSeePawn`
  (params (Pawn :type "Pawn Object Reference"))
  ;[1 1 1] Run if player is close
  (set `CharacterMovementComponent.MaxWalkSpeed` 400.0 (`self.CharacterMovement`)))

(event `self.ReceiveBeginPlay`
  ;[1 1 1] Main Event
  (`self.RunToPlayer`))

(event `RunToPlayer`
  ;[1 1 1] Chase player
  (if (not (`self.isDead`))
    (`|AIMoveTo` self (0.0 0.0 0.0) (`GameplayStatics.GetPlayerController` 0) 40.0
      (:`OnSuccess`
        (`self.AttackPlayer`))
      (:`OnFail`
        (`self.RunToPlayer`)))))

(event `AttackPlayer`
  ;[1 1 1] Attack Player
  (`|PlayMontage` (`self.Mesh`) "/Game/_Main/Enemy/Animation/Attack.Attack"
    (:`OnCompleted`
      (`self.RunToPlayer` :!label _label))
    (:`OnInterrupted`
      (goto _label))
    (:`OnNotifyBegin`
      (bind (_outactors _returnvalue) (`KismetSystemLibrary.SphereOverlapActors` (`SceneComponent.K2_GetComponentLocation` (`self.Arrow1`)) 110.0 (`|MakeArray` "ObjectTypeQuery3" :!type "EObjectTypeQuery Enum") "/Game/_Main/Blueprints/BP_FirstPersonCharacter.BP_FirstPersonCharacter_C" (`|MakeArray` self :!type "Actor Object Reference")))
      (if _returnvalue
        (for _array_element _outactors
          (`GameplayStatics.ApplyDamage` _array_element 20.0 (`self.GetController`) self "/Script/Engine.DamageType"))))))

(event `self.ReceivePointDamage`
  (params (Damage :type "Float (single-precision)") (DamageType :type "DamageType Object Reference") (HitLocation :type "Vector Structure") (HitNormal :type "Vector Structure") (HitComponent :type "PrimitiveComponent Object Reference") (BoneName :type Name) (ShotFromDirection :type "Vector Structure") (InstigatedBy :type "Controller Object Reference") (DamageCauser :type "Actor Object Reference") (HitInfo :type "HitResult Structure (by ref)"))
  ;[1 1 1] Apply Damage
  (if (`self.isDead`)
    _
    (elif (<= (`self.Health`) 0.0)
      (`self.Death`)
      (else
        (bind _output_get (set `self.Health` (- (`self.Health`) Damage)))
        (if (<= _output_get 0.0)
          (`self.Death`)
          (`PrimitiveComponent.SetCollisionResponseToChannel` (`self.CapsuleComponent`) "ECC_Pawn" "ECR_Overlap")
          (`PrimitiveComponent.SetCollisionEnabled` (`self.Mesh`) "NoCollision")
          (bind _asgame_mode_shooter (cast `/Game/_Main/Blueprints/GameModeShooter` (`GameplayStatics.GetGameMode`)))
          (`/Game/_Main/Blueprints/GameModeShooter.EnemyKilled` _asgame_mode_shooter)
          (`KismetSystemLibrary.Delay` 10.0)
          (`self.K2_DestroyActor`)
          (else
            (`|PlayMontage` (`self.Mesh`) "/Game/_Main/Enemy/Animation/HitReact_Front_Montage.HitReact_Front_Montage")))))))

(event `Death`
  (bind _mesh (`self.Mesh`))
  ;[1 1 1] Death Animation
  (set `self.isDead` true)
  (`MovementComponent.StopMovementImmediately` (`self.CharacterMovement`))
  (if (`KismetMathLibrary.RandomBool`)
    (`|PlayMontage` _mesh "/Game/_Main/Enemy/Animation/Death_B_Montage.Death_B_Montage")
    (else
      (`|PlayMontage` _mesh "/Game/_Main/Enemy/Animation/Death_A_Montage.Death_A_Montage"))))

(fn `UserConstructionScript`)